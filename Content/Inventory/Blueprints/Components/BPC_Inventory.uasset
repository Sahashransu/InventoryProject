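; BPC_Inventory is a player inventory component that also tracks money and health.
; On BeginPlay it adds the inventory input mapping, creates the inventory and health bar widgets, and binds to the player capsule's overlap.
; Overlapping BP_Money adds its DT_Money value to the inventory widget's total and destroys it; the toggle input opens the inventory in UI-only mode.
; Clamped health functions refresh the health bar, with temporary N/M test keys.
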(event `self.ReceiveBeginPlay`
  ;[1 1 1] Begin Play
  (`EnhancedInputSubsystemInterface.AddMappingContext` (pcsubsystem `EnhancedInputLocalPlayerSubsystem` (`GameplayStatics.GetPlayerController` 0)) "/Game/Inventory/Blueprints/EnhancedInput/IMC_InventoryInput.IMC_InventoryInput" 0 (struct))
  (bind _returnvalue (`|CreateWidget` "/Game/Inventory/Blueprints/Widget/WBP_Inventory.WBP_Inventory_C"))
  (set `self.WBP_Inventory` _returnvalue)
  (bind _asbp_third_person_character (cast `/Game/ThirdPerson/Blueprints/BP_ThirdPersonCharacter` (`GameplayStatics.GetPlayerCharacter` 0)))
  (bind _output_get (set `self.As BP Third Person Character` _asbp_third_person_character))
  (add `PrimitiveComponent.OnComponentBeginOverlap` (`Character.CapsuleComponent` _output_get) (`|CreateDelegate` :!event `Collide With Item`))
  (bind _returnvalue_2 (`|CreateWidget` "/Game/Inventory/Blueprints/Widget/WBP_HealthBar.WBP_HealthBar_C"))
  (bind _output_get_2 (set `self.WBP_HealthBar` _returnvalue_2))
  (`UserWidget.SetPositionInViewport` _output_get_2 (5.0 10.0) true)
  (`UserWidget.AddToViewport` _output_get_2 0))

(event `EnhancedInput|/Game/Inventory/Blueprints/EnhancedInput/IA_InventoryToggle`
  (params (ActionValue :type Boolean) (ElapsedSeconds :type "Float (double-precision)") (TriggeredSeconds :type "Float (double-precision)") (InputAction :type "InputAction Object Reference" :default "/Game/Inventory/Blueprints/EnhancedInput/IA_InventoryToggle.IA_InventoryToggle"))
  (bind _returnvalue (`GameplayStatics.GetPlayerController` 0))
  ;[1 1 1] Opening Inventory
  (:`Triggered`
    (`UserWidget.AddToViewport` (`self.WBP_Inventory`) 0)
    (set `PlayerController.bShowMouseCursor` true _returnvalue)
    (`WidgetBlueprintLibrary.SetInputMode_UIOnlyEx` _returnvalue (`self.WBP_Inventory`))))

(event `Collide With Item`
  (params (OverlappedComponent :type "PrimitiveComponent Object Reference") (OtherActor :type "Actor Object Reference") (OtherComp :type "PrimitiveComponent Object Reference") (OtherBodyIndex :type Integer) (bFromSweep :type Boolean) (SweepResult :type "HitResult Structure (by ref)"))
  ;[1 1 1] Gaining Money
  (bind _asbp_money (cast `/Game/Inventory/Blueprints/Actors/BP_Money` OtherActor))
  (bind (_dt_money_datatable _dt_money_rowname) (break `DataTableRowHandle` (`/Game/Inventory/Blueprints/Actors/BP_Money.DT_Money` _asbp_money)))
  (bind _returnvalue (`|GetDataTableRow` "/Game/Inventory/Blueprints/DataTables/DT_Money.DT_Money" _dt_money_rowname)
    (:`then`
      (set `self.MoneyGained` (+ (`.Value_5_C961F86B45CF643DBC22F9A33AF11877` (break `/Game/Inventory/Blueprints/Structs/Struct_Money` _returnvalue)) (`self.MoneyGained`)))
      (set `/Game/Inventory/Blueprints/Widget/WBP_Inventory.MoneyAmount` (`self.MoneyGained`) (`self.WBP_Inventory`))
      (`Actor.K2_DestroyActor` _asbp_money))))

(event `Key|N`
  (params (Key :type "Key Structure"))
  ;[1 1 1] Temp
  (:`Pressed`
    (`self.IncreaseHealth` 0.5)))

(event `Key|M`
  (params (Key :type "Key Structure"))
  ;[1 1 1] Temp
  (:`Pressed`
    (`self.DecreaseHealth` 0.5)))

(fn `DecreaseHealth`
  (params (`Health to Decrease` :type "Float (double-precision)"))
  (bind _returnvalue (- (`self.Health`) `Health to Decrease`))
  (if (<= _returnvalue 0.0)
    (set `self.Health` 0.0)
    (else
      (set `self.Health` _returnvalue)))
  (`/Game/Inventory/Blueprints/Widget/WBP_HealthBar.UpdateHealth` (`self.WBP_HealthBar`)))

(fn `IncreaseHealth`
  (params (`Health to Increase` :type "Float (double-precision)"))
  (bind _returnvalue (+ `Health to Increase` (`self.Health`)))
  (if (>= _returnvalue (`self.MaxHealth`))
    (set `self.Health` (`self.MaxHealth`))
    (else
      (set `self.Health` _returnvalue)))
  (`/Game/Inventory/Blueprints/Widget/WBP_HealthBar.UpdateHealth` (`self.WBP_HealthBar`)))